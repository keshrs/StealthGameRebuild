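; Cinematic controller that fades the view in when play begins, using a FadeSequence level sequence.
; FadeIn and FadeToBlack each create a new sequence player and play a different frame range of that same sequence.
; Only FadeIn runs; the chain that fades to black, waits and fades back in is unconnected, and IntroAnimation is unused.
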(event `self.ReceiveBeginPlay`
  (`self.FadeIn`))

(fn `FadeIn`
  (bind _outactor (`LevelSequencePlayer.CreateLevelSequencePlayer` (`self.FadeSequence`)))
  (`MovieSceneSequencePlayer.SetFrameRange` (`LevelSequenceActor.SequencePlayer` _outactor) 0 80)
  (`MovieSceneSequencePlayer.Play` (`LevelSequenceActor.SequencePlayer` _outactor)))

(fn `FadeToBlack`
  (bind _outactor (`LevelSequencePlayer.CreateLevelSequencePlayer` (`self.FadeSequence`)))
  (`MovieSceneSequencePlayer.SetFrameRange` (`LevelSequenceActor.SequencePlayer` _outactor) 150 190)
  (`MovieSceneSequencePlayer.Play` (`LevelSequenceActor.SequencePlayer` _outactor)))

(fn `UserConstructionScript`)