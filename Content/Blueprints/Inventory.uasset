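; Player inventory actor that tracks keycards, the level-exit Buzzcard and pistol ammo.
; AddItem identifies pickups by object-name substring, sets card flags or adds capped ammo, and shows a message through the player character's UI.
; GetBullet draws down the six-round magazine and total ammo together, while Reload refills it from that total.
; ClearCards omits the green card and ResetCardsForNextLevel omits the blue.
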(event `self.ReceiveBeginPlay`
  (`self.Reload`))

(fn `AddItem`
  (params (NewItem :type "/Game/Blueprints/Item Object Reference"))
  (returns (WasAdded :type Boolean) (ItemGetMessage :type String))
  (bind _returnvalue (`KismetSystemLibrary.GetObjectName` NewItem))
  (bind _pistolammomax (`self.PistolAmmoMax`))
  (bind _returnvalue_2 (`KismetStringLibrary.Contains` _returnvalue "Ammo"))
  (bind _returnvalue_3 (`KismetStringLibrary.Contains` _returnvalue "BuzzCard"))
  (bind _returnvalue_4 (`KismetStringLibrary.Contains` _returnvalue "Red"))
  (bind _returnvalue_5 (`KismetStringLibrary.Contains` _returnvalue "Blue"))
  (bind _returnvalue_6 (`KismetStringLibrary.Contains` _returnvalue "Green"))
  (bind _returnvalue_7 (+ (`self.CurrPistolAmmo`) 10))
  (bind _returnvalue_8 (or _returnvalue_5 _returnvalue_4 _returnvalue_6 _returnvalue_3 _returnvalue_2))
  (if _returnvalue_3
    (set `self.Buzzcard` true)
    (set `self.Message` "Buzzcard acquired! \nMove to the next floor!")
    (set `self.TimeToDisplay` 5.0)
    (elif _returnvalue_4
      (set `self.RedCard` true)
      (set `self.Message` "Acquired Keycard!" :!label _label)
      (set `self.TimeToDisplay` 1.5)
      (elif _returnvalue_5
        (set `self.BlueCard` true)
        (goto _label)
        (elif _returnvalue_6
          (set `self.GreenCard` true)
          (goto _label)
          (elif _returnvalue_2
            (set `self.CurrPistolAmmo` (select `bool` (> _returnvalue_7 _pistolammomax) :`false` _returnvalue_7 :`true` _pistolammomax))
            (set `self.Message` "Got 10 Ammo")
            (set `self.TimeToDisplay` 1.5))))))
  (if _returnvalue_8
    (bind _asmc (cast `/Game/Characters/mainCharacter/mc` (`GameplayStatics.GetPlayerCharacter` 0)))
    (`/Game/UI/HealthAmmoUI.ShowMessage` (`/Game/Characters/mainCharacter/mc.AmmoHealthUI` _asmc) (`self.Message`) (`self.TimeToDisplay`)))
  (return _returnvalue_8 (`self.Message`)))

(fn `ClearCards`
  (set `self.Buzzcard` false)
  (set `self.BlueCard` false)
  (set `self.RedCard` false))

(fn `GetBullet`
  (returns (NewParam :type Boolean))
  (bind _returnvalue (> (`self.BulletsLoaded`) 0))
  (if _returnvalue
    (`/Engine/EditorBlueprintResources/StandardMacros.DecrementInt` (`self.BulletsLoaded`)
      (:`  `
        (`/Engine/EditorBlueprintResources/StandardMacros.DecrementInt` (`self.CurrPistolAmmo`)
          (:`  `
            _)))))
  (return _returnvalue))

(fn `Initalize`
  (set `self.CurrPistolAmmo` (`self.PistolAmmoMax`))
  (`self.ClearCards`))

(fn `Reload`
  (set `self.BulletsLoaded` (`KismetMathLibrary.Min` (`self.CurrPistolAmmo`) 6)))

(fn `ResetCardsForNextLevel`
  (set `self.Buzzcard` false)
  (set `self.RedCard` false)
  (set `self.GreenCard` false)
  (set `self.BulletsLoaded` 6))

(fn `UserConstructionScript`)