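; Setup actor that applies optional display overrides through console commands when its custom event is called.
; One flag switches the view mode to unlit, disabling lighting.
; A second flag builds an r.SetRes fullscreen command by appending the configurable X and Y resolution to a string variable, then executes it.
; The construction script is empty, and nothing in the file calls the event.
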(event `CustomEvent`
  (if (`self.DiableLighting`)
    (`KismetSystemLibrary.ExecuteConsoleCommand` "viewmode unlit" null))
  (if (`self.LowResolution`)
    (`KismetSystemLibrary.ExecuteConsoleCommand` (`KismetStringLibrary.Concat_StrStr` (`KismetStringLibrary.Concat_StrStr` (`KismetStringLibrary.Concat_StrStr` (`KismetStringLibrary.Concat_StrStr` (`KismetStringLibrary.Concat_StrStr` (`self.NewVar_0`) "r.SetRes ") (`KismetStringLibrary.Conv_IntToString` (`self.ResX`))) "x") (`KismetStringLibrary.Conv_IntToString` (`self.ResY`))) "f") null)))

(fn `UserConstructionScript`)