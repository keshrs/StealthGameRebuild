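; Player camera actor that switches the view between first and third person.
; On BeginPlay it registers with the mc pawn, makes its FollowAtOffset parent follow that pawn and requests an immediate third-person view.
; SetFirstPerson either teleports the camera or blends the controller's view target to the pawn (first person) or the parent's first attached actor (third person).
; Rotation alignment for first person is an unconnected TODO.
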(event `self.ReceiveBeginPlay`
  (bind _returnvalue (`ActorComponent.GetOwner` (`SceneComponent.GetAttachParent` (`self.SceneComponent`))))
  (set `self.Parent` _returnvalue)
  (bind _asmc (cast `/Game/Characters/mainCharacter/mc` (`GameplayStatics.GetPlayerPawn` 0)))
  (`/Game/Characters/mainCharacter/mc.SetCamera` _asmc self)
  (set `self.FPS_Position` (`GameplayStatics.GetPlayerPawn` 0))
  (set `self.TPS_Position` (`|GetArrayItem` (`self.GetAttachedActors` _returnvalue)))
  (bind _asfollow_at_offset_blueprint (cast `/Game/Blueprints/FollowAtOffset_Blueprint` (`self.Parent`)))
  (`/Game/Blueprints/FollowAtOffset_Blueprint.SetFollowTarget` _asfollow_at_offset_blueprint (`GameplayStatics.GetPlayerPawn` 0))
  (bind _asmc_2 (cast `/Game/Characters/mainCharacter/mc` (`GameplayStatics.GetPlayerPawn` 0)))
  (`/Game/Characters/mainCharacter/mc.SetFirstPerson` _asmc_2 false true))

(event `self.ReceiveTick`
  (params (DeltaSeconds :type "Float (single-precision)")))

(fn `SetFirstPerson`
  (params (IsFirstPerson :type Boolean) (Immediate :type Boolean) (BodyMeshRotation :type "Rotator Structure"))
  (bind _returnvalue (`GameplayStatics.GetPlayerController` 0))
  (bind _fps_position (`self.FPS_Position`))
  (bind _tps_position (`self.TPS_Position`))
  (if Immediate
    (if IsFirstPerson
      (`self.K2_SetActorLocation` (`self.K2_GetActorLocation` _fps_position))
      (`self.K2_SetActorRotation` (`self.K2_GetActorRotation` _fps_position))
      (else
        (`self.K2_SetActorLocation` (`self.K2_GetActorLocation` _tps_position))
        (`self.K2_SetActorRotation` (`self.K2_GetActorRotation` _tps_position))))
    (elif IsFirstPerson
      (if (not (`self.HasRotatedYet`))
        (set `self.HasRotatedYet` true))
      (`PlayerController.SetViewTargetWithBlend` _returnvalue (`self.FPS_Position`) 0.25 "VTBlend_Linear" 0.0 false)
      (else
        (`PlayerController.SetViewTargetWithBlend` _returnvalue (`self.TPS_Position`) 0.25 "VTBlend_Linear" 0.0 false)))))

(fn `UserConstructionScript`)