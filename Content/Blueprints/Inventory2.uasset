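; Inventory2 is an inventory Blueprint that tracks pistol ammo and three keycard flags: Buzzcard, BlueCard and RedCard.
; Initalize refills pistol ammo to its maximum and calls ClearCards to reset every card flag.
; AddItem identifies items by object-name substring, setting Buzzcard or RedCard and returning whether the name contains "Red".
; AddItem has no branch for BlueCard, and the event graph is empty.
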(fn `AddItem`
  (params (NewItem :type "/Game/Blueprints/Item Object Reference"))
  (returns (WasAdded :type Boolean))
  (bind _returnvalue (`KismetSystemLibrary.GetObjectName` NewItem))
  (bind _returnvalue_2 (`KismetStringLibrary.Contains` _returnvalue "Red"))
  (if (`KismetStringLibrary.Contains` _returnvalue "BuzzCard")
    (set `self.Buzzcard` true)
    (return _returnvalue_2)
    (elif _returnvalue_2
      (set `self.RedCard` true)
      (return _returnvalue_2))))

(fn `ClearCards`
  (set `self.Buzzcard` false)
  (set `self.BlueCard` false)
  (set `self.RedCard` false))

(fn `Initalize`
  (set `self.CurrPistolAmmo` (`self.PistolAmmoMax`))
  (`self.ClearCards`))

(fn `UserConstructionScript`)