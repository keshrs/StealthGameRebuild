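; Actor that plays the game's intro and ending text cutscenes as fullscreen widgets with FadeIn animations, muting the background music for each.
; The intro starts on BeginPlay; when its animation finishes, it hides the widget, restores the music and enables player control.
; Tick polls a PlayEndCutscene flag to start the ending, whose animation-finished event enables control, hides both widgets and opens MainMenu.
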(event `self.ReceiveBeginPlay`
  (bind _introcutscene (`self.IntroCutscene`))
  (bind _fadein (`/Game/UI/IntroCutsceneText.FadeIn` _introcutscene))
  (bind _outactors (`GameplayStatics.GetAllActorsOfClass` "/Game/Blueprints/BackgroundMusic.BackgroundMusic_C"))
  (`/Game/Blueprints/BackgroundMusic.ChangeVolume` (`|GetArrayItem` _outactors) 0.0)
  (bind _returnvalue (`|CreateWidget` "/Game/UI/IntroCutsceneText.IntroCutsceneText_C"))
  (bind _output_get (set `self.IntroCutscene` _returnvalue))
  (`UserWidget.AddToViewport` _introcutscene 0)
  (`UserWidget.AddToViewport` _output_get 0)
  (`UserWidget.PlayAnimation` _introcutscene _fadein 0.0 1 "Forward" 1.0)
  (add `WidgetAnimation.OnAnimationFinished` _fadein (delegate `OnCutsceneFinished`)))

(event `OnCutsceneFinished`
  (bind _asmc (cast `/Game/Characters/mainCharacter/mc` (`GameplayStatics.GetPlayerCharacter` 0)))
  (`/Game/Characters/mainCharacter/mc.EnableControl` _asmc)
  (`Widget.SetVisibility` (`self.IntroCutscene`) "Hidden")
  (bind _outactors (`GameplayStatics.GetAllActorsOfClass` "/Game/Blueprints/BackgroundMusic.BackgroundMusic_C"))
  (`/Game/Blueprints/BackgroundMusic.ChangeVolume` (`|GetArrayItem` _outactors) 1.0))

(event `self.ReceiveTick`
  (params (DeltaSeconds :type "Float (single-precision)"))
  (bind _endcutscene (`self.EndCutscene`))
  (bind _fadein (`/Game/UI/EndCutsceneText.FadeIn` _endcutscene))
  (if (`self.PlayEndCutscene`)
    (set `self.PlayEndCutscene` false)
    (bind _outactors (`GameplayStatics.GetAllActorsOfClass` "/Game/Blueprints/BackgroundMusic.BackgroundMusic_C"))
    (`/Game/Blueprints/BackgroundMusic.ChangeVolume` (`|GetArrayItem` _outactors) 0.0)
    (bind _returnvalue (`|CreateWidget` "/Game/UI/EndCutsceneText.EndCutsceneText_C"))
    (set `self.EndCutscene` _returnvalue)
    (`UserWidget.AddToViewport` _endcutscene 0)
    (`UserWidget.PlayAnimation` _endcutscene _fadein 0.0 1 "Forward" 1.0)
    (add `WidgetAnimation.OnAnimationFinished` _fadein (delegate `CustomEvent`))))

(event `CustomEvent`
  (bind _asmc (cast `/Game/Characters/mainCharacter/mc` (`GameplayStatics.GetPlayerCharacter` 0)))
  (`/Game/Characters/mainCharacter/mc.EnableControl` _asmc)
  (`Widget.SetVisibility` (`self.IntroCutscene`) "Hidden")
  (`Widget.SetVisibility` (`self.EndCutscene`) "Hidden")
  (`GameplayStatics.OpenLevel` "MainMenu"))

(fn `UserConstructionScript`)