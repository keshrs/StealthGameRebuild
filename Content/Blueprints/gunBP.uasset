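; Gun actor that the player character carries, with a Shoot function that produces a muzzle smoke effect.
; On BeginPlay it attaches to the player mesh's WeaponHolder socket and stores itself in the mc character's Gun variable.
; Shoot spawns a flipbook barrel effect actor, attaches it to the gun's static mesh, then applies a hardcoded offset and rotation.
; Shoot is purely visual, with no projectile, trace or damage.
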(event `self.ReceiveBeginPlay`
  (bind _returnvalue (`GameplayStatics.GetPlayerCharacter` 0))
  (`self.K2_AttachToComponent` (`Character.Mesh` _returnvalue) "WeaponHolder" "KeepRelative" "KeepRelative" "KeepRelative")
  (bind _asmc (cast `/Game/Characters/mainCharacter/mc` _returnvalue))
  (set `/Game/Characters/mainCharacter/mc.Gun` self _asmc))

(fn `Shoot`
  (bind _gunsmoke (`self.Gunsmoke`))
  (bind _returnvalue (`|SpawnActorFromClass` "/Game/Blueprints/Gun_barrel_effect_flipbook_Blueprint.Gun_barrel_effect_flipbook_Blueprint_C" (`SceneComponent.GetRelativeTransform` (`self.Barrel`)) "Undefined" "OverrideRootScale" self null))
  (bind _output_get (set `self.Gunsmoke` _returnvalue))
  (`self.K2_AttachToComponent` _output_get (`self.StaticMesh`) "WeaponHolder" "SnapToTarget" "SnapToTarget" "KeepWorld" true)
  (`SceneComponent.K2_AddRelativeLocation` (`PaperFlipbookActor.RenderComponent` (`self.Gunsmoke`)) (-15.0 160.0 30.0) false false)
  (`self.K2_SetActorRotation` _gunsmoke (`KismetMathLibrary.Conv_VectorToRotator` (`KismetMathLibrary.GreaterGreater_VectorRotator` (90.0 0.0 0.0) (`self.K2_GetActorRotation` _gunsmoke))) false))

(fn `UserConstructionScript`)