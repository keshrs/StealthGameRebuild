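; Level manager actor that streams levels from an ordered list, loading the first on BeginPlay unless starting in a test area.
; Next and reload functions set flags that Tick consumes to load and unload streamed levels asynchronously.
; Reloading also calls Respawn on the player's mc character.
; LoadPrevLevel's bounds check is inverted, so from any valid index it restores the index without loading.
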(event `self.ReceiveBeginPlay`
  (bind _output (`|GetArrayItem` (`self.LevelOrder`)))
  ;[1 1 1] Load into the starting area
  (if (not (`self.StartInTestArea`))
    (`GameplayStatics.LoadStreamLevel` _output true)
    (set `self.LastLevel` _output)))

(event `InputAction|Interact`
  (params (Key :type "Key Structure")))

(event `self.ReceiveTick`
  (params (DeltaSeconds :type "Float (single-precision)"))
  (bind _output (`|GetArrayItem` (`self.LevelOrder`) (`self.CurrentLevelIndex`)))
  (bind _output_2 (`|GetArrayItem` (`self.LevelOrder`) (`self.CurrentLevelIndex`)))
  (if (`self.ReadyToLoad`)
    (set `self.ReadyToLoad` false)
    (if (`self.Reload`)
      (set `self.Reload` false)
      (`GameplayStatics.UnloadStreamLevel` _output)
      (`GameplayStatics.LoadStreamLevel` _output true)
      (bind _asmc (cast `/Game/Characters/mainCharacter/mc` (`GameplayStatics.GetPlayerCharacter` 0)))
      (`/Game/Characters/mainCharacter/mc.Respawn` _asmc)
      (else
        (`GameplayStatics.LoadStreamLevel` _output_2 true)
        (`GameplayStatics.UnloadStreamLevel` (`self.LastLevel`))
        (set `self.LastLevel` _output_2)))))

(fn `LoadNextLevel`
  (`/Engine/EditorBlueprintResources/StandardMacros.IncrementInt` (`self.CurrentLevelIndex`)
    (:`  `
      (if (not (>= (`self.CurrentLevelIndex`) (`KismetArrayLibrary.Array_Length` (`self.LevelOrder`))))
        (set `self.ReadyToLoad` true)
        (else
          ;[1 1 1] We  are already at the last level so we can't go up
          (`/Engine/EditorBlueprintResources/StandardMacros.DecrementInt` (`self.CurrentLevelIndex`)))))))

(fn `LoadPrevLevel`
  (`/Engine/EditorBlueprintResources/StandardMacros.DecrementInt` (`self.CurrentLevelIndex`)
    (:`  `
      (if (not (>= (`self.CurrentLevelIndex`) -1))
        (set `self.ReadyToLoad` true)
        (else
          ;[1 1 1] We  are already at the last level so we can't go up
          (`/Engine/EditorBlueprintResources/StandardMacros.IncrementInt` (`self.CurrentLevelIndex`)))))))

(fn `ReloadCurrentLevel`
  (set `self.ReadyToLoad` true)
  (set `self.Reload` true))

(fn `UserConstructionScript`)