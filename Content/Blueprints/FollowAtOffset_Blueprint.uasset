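; An actor Blueprint that follows a target actor at a fixed offset once SetFollowTarget assigns one.
; Each Tick it moves to the target's location plus a world-space Offset, without sweeping.
; When UseTargetRotation is set, it also faces along the target's forward vector plus the Rotation value, added as a vector before conversion back to a rotator.
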(event `self.ReceiveTick`
  (params (DeltaSeconds :type "Float (single-precision)"))
  (bind _followtarget (`self.FollowTarget`))
  (if (`self.IsFollowing`)
    (`self.K2_SetActorLocation` (+ (`self.K2_GetActorLocation` _followtarget) (`self.Offset`)))
    (if (`self.UseTargetRotation`)
      (`self.K2_SetActorRotation` (`KismetMathLibrary.Conv_VectorToRotator` (+ (`self.Rotation`) (`KismetMathLibrary.Conv_RotatorToVector` (`self.K2_GetActorRotation` _followtarget))))))))

(fn `SetFollowTarget`
  (params (FollowTarget :type "Actor Object Reference"))
  (set `self.FollowTarget` FollowTarget)
  (set `self.IsFollowing` true))

(fn `UserConstructionScript`)