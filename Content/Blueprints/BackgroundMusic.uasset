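; Background music actor that switches tracks based on whether any enemies have spotted the player.
; Spotted and unspotted events maintain a list of enemies, triggering the alert track when the first is added and a chase-end transition when the last is removed.
; When audio finishes, alert advances to chase and chase end to sneak.
; ChangeSound maps the current state to a sound and volume multiplier, then restarts playback.
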(event `EventSpotted`
  (params (enemy :type "Actor Object Reference"))
  (bind _spottedactors (`self.spottedActors`))
  (bind _output_get (set `self.prevSetLength` (`BlueprintSetLibrary.Set_Length` _spottedactors)))
  (`BlueprintSetLibrary.Set_Add` _spottedactors enemy)
  (if (and (> (`BlueprintSetLibrary.Set_Length` _spottedactors) 0) (== _output_get 0))
    (set `self.backgroundState` "alert")
    (`self.changeSound`)))

(event `EventUnspotted`
  (params (enemy :type "Actor Object Reference"))
  (bind _spottedactors (`self.spottedActors`))
  (bind _output_get (set `self.prevSetLength` (`BlueprintSetLibrary.Set_Length` _spottedactors)))
  (`BlueprintSetLibrary.Set_Remove` _spottedactors enemy)
  (if (and (== (`BlueprintSetLibrary.Set_Length` _spottedactors) 0) (> _output_get 0))
    (set `self.backgroundState` "chaseEnd")
    (`self.changeSound`)))

(event `self.varBackgroundMusic.OnAudioFinished`
  (switch `string` (`self.backgroundState`)
    (:`Default`
      _)
    (:`alert`
      (set `self.backgroundState` "chase"))
    (:`chaseEnd`
      (set `self.backgroundState` "sneak")))
  (`self.changeSound`))

(event `self.ReceiveBeginPlay`
  (`self.changeSound`))

(fn `changeSound`
  (bind _varbackgroundmusic (`self.varBackgroundMusic`))
  (bind _varbackgroundmusic_2 (`self.varBackgroundMusic`))
  (switch `string` (`self.backgroundState`)
    (:`Default`
      (`AudioComponent.SetSound` _varbackgroundmusic_2 (`self.SneakMusic`) :!label _label)
      (`AudioComponent.SetVolumeMultiplier` _varbackgroundmusic (`self.sneakMusicMultiplier`)))
    (:`sneak`
      (goto _label))
    (:`alert`
      (`AudioComponent.SetSound` _varbackgroundmusic_2 (`self.Alert`))
      (`AudioComponent.SetVolumeMultiplier` _varbackgroundmusic (`self.alertMusicMultiplier`)))
    (:`chase`
      (`AudioComponent.SetSound` _varbackgroundmusic_2 (`self.ChaseMusic`))
      (`AudioComponent.SetVolumeMultiplier` _varbackgroundmusic (`self.chaseMusicMultiplier`)))
    (:`chaseEnd`
      (`AudioComponent.SetSound` _varbackgroundmusic_2 (`self.ChaseEndTransition`))
      (`AudioComponent.SetVolumeMultiplier` _varbackgroundmusic (`self.chaseEndTransitionMultiplier`))))
  (`AudioComponent.Play` _varbackgroundmusic_2 0.0))

(fn `UserConstructionScript`)